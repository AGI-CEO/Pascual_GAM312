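; Player character Blueprint that creates the player HUD and handles opening and closing the crafting menu.
; On BeginPlay it creates Player_W, stores it as PlayerUI and adds it to the viewport.
; The CraftMenu input uses a FlipFlop to alternately add a new CraftingW with mouse cursor and Game-and-UI input, or remove it and return focus to game-only input.
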(event EventBeginPlay
  (bind _returnvalue (UserInterface|CreateWidget "/Game/Widgets/Player_W.Player_W_C"))
  (bind _output_get (Variables|Default|SetPlayerUI _returnvalue))
  (UserInterface|Viewport|AddtoViewport _output_get 0))

(event Collision|EventActorBeginOverlap
  (params (OtherActor :type Actor%20Object%20Reference)))

(event EventTick
  (params (DeltaSeconds :type Float%20%28single-precision%29)))

(event Input|ActionEvents|InputActionCraftMenu
  (params (Key :type Key%20Structure :default "None"))
  (bind _returnvalue (Game|GetPlayerController 0))
  (:Pressed
    (Utilities|FlowControl|FlipFlop
      (:A
        (bind _returnvalue_2 (UserInterface|CreateWidget "/Game/Widgets/CraftingW.CraftingW_C"))
        (UserInterface|Viewport|AddtoViewport _returnvalue_2 0)
        (Variables|/Script/Engine.PlayerController|SetbShowMouseCursor _returnvalue true)
        (Input|SetInputModeGameandUI _returnvalue _returnvalue_2 "DoNotLock" true false))
      (:B
        (Widget|RemovefromParent _returnvalue_2)
        (Variables|/Script/Engine.PlayerController|SetbShowMouseCursor _returnvalue false)
        (Input|SetInputModeGameOnly _returnvalue false)
        (Class|WidgetBlueprintLibrary|SetFocustoGameViewport)))))

(fn ConstructionScript)